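; BP_AlertLight is a spotlight hazard that alerts smart enemy AI when the third-person character overlaps its static mesh while the light is visible.
; The overlap loops over every BP_SmartEnemyAI, clears BeenSeen on its AIC_Smart controller and calls BroadcastAlert.
; ToggleLight stores the linked button, hides the light for a fixed delay, then restores it and turns that button's cube green.
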(event `self.ReceiveBeginPlay`
  (`SceneComponent.SetVisibility` (`self.SpotLight`) true false))

(event `self.StaticMesh.OnComponentBeginOverlap`
  (params (OverlappedComponent :type "PrimitiveComponent Object Reference") (OtherActor :type "Actor Object Reference") (OtherComp :type "PrimitiveComponent Object Reference") (OtherBodyIndex :type Integer) (bFromSweep :type Boolean) (SweepResult :type "HitResult Structure (by ref)"))
  (cast `/Game/ThirdPerson/Blueprints/BP_ThirdPersonCharacter` OtherActor)
  (if (`SceneComponent.IsVisible` (`self.SpotLight`))
    (bind _outactors (`GameplayStatics.GetAllActorsOfClass` "/Game/Blueprints/BP_SmartEnemyAI.BP_SmartEnemyAI_C"))
    (for _array_element _outactors
      (bind _asai_controller (cast `/Game/Blueprints/AIC_Smart` (`Pawn.GetController` _array_element)))
      (set `/Game/Blueprints/AIC_Smart.BeenSeen` false _asai_controller)
      (`/Game/Blueprints/AIC_Smart.BroadcastAlert` _asai_controller))))

(event `ToggleLight`
  (params (LinkedButtton :type "/Game/Blueprints/BP_LightSwitch Object Reference"))
  (set `self.CurrentButton` LinkedButtton)
  (`SceneComponent.SetVisibility` (`self.SpotLight`) false false)
  (`KismetSystemLibrary.Delay` 5.0)
  (`SceneComponent.SetVisibility` (`self.SpotLight`) true false)
  (`PrimitiveComponent.SetMaterial` (`/Game/Blueprints/BP_LightSwitch.Cube` (`self.CurrentButton`)) 0 "/Game/Green.Green"))

(fn `UserConstructionScript`)