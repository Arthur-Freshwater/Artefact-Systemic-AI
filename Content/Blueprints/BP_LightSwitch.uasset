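; BP_LightSwitch is an interactable switch that toggles its linked light.
; A box overlap registers the switch as the third-person character's current one, sets that character's CanSwitchLight flag and shows a widget; leaving clears the flag and hides it.
; PressButton calls ToggleLight on LinkedLight, passing itself, and turns the cube red, while ResetButton turns it green.
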(event `self.ReceiveBeginPlay`
  (`SceneComponent.SetVisibility` (`self.Widget`) false false))

(event `self.Box.OnComponentBeginOverlap`
  (params (OverlappedComponent :type "PrimitiveComponent Object Reference") (OtherActor :type "Actor Object Reference") (OtherComp :type "PrimitiveComponent Object Reference") (OtherBodyIndex :type Integer) (bFromSweep :type Boolean) (SweepResult :type "HitResult Structure (by ref)"))
  (bind _asbp_third_person_character (cast `/Game/ThirdPerson/Blueprints/BP_ThirdPersonCharacter` OtherActor))
  (set `/Game/ThirdPerson/Blueprints/BP_ThirdPersonCharacter.CurrentLightSwitch` self _asbp_third_person_character)
  (bind _output_get (set `/Game/ThirdPerson/Blueprints/BP_ThirdPersonCharacter.CanSwitchLight` true _asbp_third_person_character))
  (`SceneComponent.SetVisibility` (`self.Widget`) _output_get false))

(event `self.Box.OnComponentEndOverlap`
  (params (OverlappedComponent :type "PrimitiveComponent Object Reference") (OtherActor :type "Actor Object Reference") (OtherComp :type "PrimitiveComponent Object Reference") (OtherBodyIndex :type Integer))
  (bind _asbp_third_person_character (cast `/Game/ThirdPerson/Blueprints/BP_ThirdPersonCharacter` OtherActor))
  (bind _output_get (set `/Game/ThirdPerson/Blueprints/BP_ThirdPersonCharacter.CanSwitchLight` false _asbp_third_person_character))
  (`SceneComponent.SetVisibility` (`self.Widget`) _output_get false))

(event `PressButton`
  (`/Game/Blueprints/BP_SpotLight.ToggleLight` (`self.LinkedLight`) self)
  (`PrimitiveComponent.SetMaterial` (`self.Cube`) 0 "/Game/Colours/Red.Red"))

(event `ResetButton`
  (`PrimitiveComponent.SetMaterial` (`self.Cube`) 0 "/Game/Colours/Green.Green"))

(fn `UserConstructionScript`)