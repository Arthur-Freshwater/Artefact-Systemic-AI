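; StateTree task for an AI's chase state that raises an alarm if the state stays active for three seconds.
; On enter it caches the player character and starts a timer, which marks the AI as having seen the player and broadcasts an alert through the AI reference.
; On exit it cancels the timer and clears the seen flag, so leaving early prevents the alert.
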(event `self.ReceiveLatentEnterState`
  (params (Transition :type "StateTreeTransitionResult Structure (by ref)"))
  (`parent.ReceiveLatentEnterState` Transition)
  (set `self.Player` (`GameplayStatics.GetPlayerCharacter` 0))
  (bind _returnvalue (`KismetSystemLibrary.K2_SetTimerDelegate` (delegate `TriggerAlarm`) 3.0))
  (set `self.AlertTimer` _returnvalue))

(event `TriggerAlarm`
  (bind _airef (`self.AIRef`))
  (set `/Game/Blueprints/Enemy/AIC_Smart.BeenSeen` true _airef)
  (`/Game/Blueprints/Enemy/AIC_Smart.BroadcastAlert` _airef))

(event `self.ReceiveExitState`
  (params (Transition :type "StateTreeTransitionResult Structure (by ref)"))
  (`KismetSystemLibrary.K2_ClearAndInvalidateTimerHandle` (`self.AlertTimer`))
  (set `/Game/Blueprints/Enemy/AIC_Smart.BeenSeen` false (`self.AIRef`)))