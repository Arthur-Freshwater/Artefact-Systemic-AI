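; GetMoveLocation is a StateTree task that supplies an AI with its next patrol destination.
; On state entry it writes the location of the BP_PatrolPoint at AIRef's CurrentPatrolPoint index into the MoveToLocation property reference.
; It then increments the index, resetting only when already at or beyond the point count, and finishes successfully, or fails if the reference is invalid.
; Point order comes from GetAllActorsOfClass, with debug prints of index and count.
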(event `self.ReceiveLatentEnterState`
  (params (Transition :type "StateTreeTransitionResult Structure (by ref)"))
  (bind _currentpatrolpoint (`/Game/Blueprints/AI_Controller.CurrentPatrolPoint` (`self.AIRef`)))
  (bind _outactors (`GameplayStatics.GetAllActorsOfClass` "/Game/Blueprints/BP_PatrolPoint.BP_PatrolPoint_C"))
  (`KismetSystemLibrary.PrintString` (`KismetStringLibrary.Conv_IntToString` _currentpatrolpoint))
  (bind _reference (`|StateTreeBlueprintPropertyRef` (`self.MoveToLocationPropertyRef`))
    (:`Succeeded`
      (`|VariableSetRef` _reference (`Actor.K2_GetActorLocation` (`|GetArrayItem` _outactors _currentpatrolpoint)))
      (bind _outactors_2 (`GameplayStatics.GetAllActorsOfClass` "/Game/Blueprints/BP_PatrolPoint.BP_PatrolPoint_C"))
      (bind _returnvalue (`KismetArrayLibrary.Array_Length` _outactors_2))
      (`KismetSystemLibrary.PrintString` (`KismetStringLibrary.Conv_IntToString` _returnvalue))
      (if (>= (`/Game/Blueprints/AI_Controller.CurrentPatrolPoint` (`self.AIRef`)) _returnvalue)
        (set `/Game/Blueprints/AI_Controller.CurrentPatrolPoint` 0 (`self.AIRef`))
        (else
          (bind _result (`/Engine/EditorBlueprintResources/StandardMacros.IncrementInt` (`/Game/Blueprints/AI_Controller.CurrentPatrolPoint` (`self.AIRef`)))
            (:`  `
              (set `/Game/Blueprints/AI_Controller.CurrentPatrolPoint` _result (`self.AIRef`))))))
      (`self.FinishTask` true))
    (:`Failed`
      (`self.FinishTask` false))))