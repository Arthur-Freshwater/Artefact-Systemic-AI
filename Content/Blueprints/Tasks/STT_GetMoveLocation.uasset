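; StateTree task that feeds a patrolling BP_SmartEnemyAI its next move destination.
; On entering the state, it writes the location of the current PatrolRoute actor into a bound MoveToLocation property reference.
; It then advances the AI's CurrentPatrolPoint, wrapping to the first point after the last, and finishes successfully.
; It fails if the property reference cannot be resolved, and prints the patrol index for debugging.
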(event `self.ReceiveLatentEnterState`
  (params (Transition :type "StateTreeTransitionResult Structure (by ref)"))
  (bind _currentpatrolpoint (`/Game/Blueprints/Enemy/AIC_Smart.CurrentPatrolPoint` (`self.AIRef`)))
  (bind _asbp_smart_enemy_ai (cast `/Game/Blueprints/Enemy/BP_SmartEnemyAI` (`self.PawnRef`)))
  (`KismetSystemLibrary.PrintString` (`KismetStringLibrary.Conv_IntToString` _currentpatrolpoint))
  (bind _reference (`|StateTreeBlueprintPropertyRef` (`self.MoveToLocationPropertyRef`))
    (:`Succeeded`
      (`|VariableSetRef` _reference (`Actor.K2_GetActorLocation` (`|GetArrayItem` (`/Game/Blueprints/Enemy/BP_SmartEnemyAI.PatrolRoute` _asbp_smart_enemy_ai) _currentpatrolpoint)))
      (bind _asbp_smart_enemy_ai_2 (cast `/Game/Blueprints/Enemy/BP_SmartEnemyAI` (`self.PawnRef`)))
      (if (>= (`/Game/Blueprints/Enemy/AIC_Smart.CurrentPatrolPoint` (`self.AIRef`)) (- (`KismetArrayLibrary.Array_Length` (`/Game/Blueprints/Enemy/BP_SmartEnemyAI.PatrolRoute` _asbp_smart_enemy_ai_2)) 1))
        (set `/Game/Blueprints/Enemy/AIC_Smart.CurrentPatrolPoint` 0 (`self.AIRef`))
        (else
          (bind _result (`/Engine/EditorBlueprintResources/StandardMacros.IncrementInt` (`/Game/Blueprints/Enemy/AIC_Smart.CurrentPatrolPoint` (`self.AIRef`)))
            (:`  `
              (set `/Game/Blueprints/Enemy/AIC_Smart.CurrentPatrolPoint` _result (`self.AIRef`))))))
      (`self.FinishTask` true))
    (:`Failed`
      (`self.FinishTask` false))))