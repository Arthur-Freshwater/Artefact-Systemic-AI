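; Enemy AI controller that turns perception and gameplay events into State Tree events for patrol, chase, investigate, flee and caught states.
; Starts patrolling shortly after possession, chases the sensed player, resumes patrol on losing them, and investigates Ball-tagged stimuli.
; Light exposure triggers fleeing.
; BroadcastAlert sends the player's location to all base-enemy controllers, which show a temporary alert widget, then chase or investigate based on BeenSeen.
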(event `self.ReceivePossess`
  (params (PossessedPawn :type "Pawn Object Reference"))
  (`BrainComponent.RestartLogic` (`self.StateTreeAI`))
  (`KismetSystemLibrary.Delay` 2.0)
  (`StateTreeComponent.SendStateTreeEvent` (`self.StateTreeAI`) (make `StateTreeEvent` (struct :`TagName` "State_Patrol"))))

(event `self.AIPerception.OnTargetPerceptionUpdated`
  (params (Actor :type "Actor Object Reference") (Stimulus :type "AIStimulus Structure"))
  (bind (_age _expirationage _strength _stimuluslocation _receiverlocation _tag _bsuccessfullysensed) (break `AIStimulus` Stimulus))
  (if (not (== _tag "Ball"))
    (if (== Actor (`GameplayStatics.GetPlayerCharacter` 0))
      (if _bsuccessfullysensed
        (`StateTreeComponent.SendStateTreeEvent` (`self.StateTreeAI`) (make `StateTreeEvent` (struct :`TagName` "State_Chase")))
        (else
          (`StateTreeComponent.SendStateTreeEvent` (`self.StateTreeAI`) (make `StateTreeEvent` (struct :`TagName` "State_Patrol"))))))
    (else
      (set `self.SoundLocation` _stimuluslocation)
      (`StateTreeComponent.SendStateTreeEvent` (`self.StateTreeAI`) (make `StateTreeEvent` (struct :`TagName` "State_Investigate"))))))

(event `In Light`
  (`KismetSystemLibrary.PrintString` "In Light")
  (`StateTreeComponent.SendStateTreeEvent` (`self.StateTreeAI`) (make `StateTreeEvent` (struct :`TagName` "State_Flee"))))

(event `CaughtPlayer`
  (`KismetSystemLibrary.PrintString` "Caught")
  (`StateTreeComponent.SendStateTreeEvent` (`self.StateTreeAI`) (make `StateTreeEvent` (struct :`TagName` "State_Caught"))))

(event `Alert`
  (params (AlertLocation :type "Vector Structure") (PlayerSpotted :type Boolean))
  (bind _returnvalue (`|CreateWidget` "/Game/Blueprints/WBP/WBP_EnemyAlert.WBP_EnemyAlert_C"))
  (`UserWidget.AddToViewport` _returnvalue 0)
  (if PlayerSpotted
    (`StateTreeComponent.SendStateTreeEvent` (`self.StateTreeAI`) (make `StateTreeEvent` (struct :`TagName` "State_Chase")))
    (else
      (set `self.SoundLocation` AlertLocation)
      (`StateTreeComponent.SendStateTreeEvent` (`self.StateTreeAI`) (make `StateTreeEvent` (struct :`TagName` "State_Investigate")))))
  (`KismetSystemLibrary.Delay` 2.0)
  (`WidgetLayoutLibrary.RemoveAllWidgets`))

(event `BroadcastAlert`
  (bind _outactors (`GameplayStatics.GetAllActorsOfClass` "/Game/Blueprints/BP_BaseEnemyAI.BP_BaseEnemyAI_C"))
  (for _array_element _outactors
    (bind _asai_controller (cast `/Game/Blueprints/AI_Controller` (`Pawn.GetController` _array_element)))
    (`self.Alert` _asai_controller (`self.K2_GetActorLocation` (`GameplayStatics.GetPlayerCharacter` 0)) (`self.BeenSeen`))))

(fn `UserConstructionScript`)