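; AIC_Simple is an enemy AI controller that switches a StateTree between patrol and chase through gameplay-tag events.
; On possess it restarts the StateTree logic and sends the Patrol event after a short delay.
; AI perception updates for the player character send the Chase event.
; That branch's condition is a constant true, so its return-to-Patrol path never runs as shown.
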(event `self.ReceivePossess`
  (params (PossessedPawn :type "Pawn Object Reference"))
  (`BrainComponent.RestartLogic` (`self.StateTreeAI`))
  (`KismetSystemLibrary.Delay` 2.0)
  (`StateTreeComponent.SendStateTreeEvent` (`self.StateTreeAI`) (make `StateTreeEvent` (struct :`TagName` "State_Patrol"))))

(event `self.AIPerception.OnTargetPerceptionUpdated`
  (params (Actor :type "Actor Object Reference") (Stimulus :type "AIStimulus Structure"))
  (if (== Actor (`GameplayStatics.GetPlayerCharacter` 0))
    (if true
      (`StateTreeComponent.SendStateTreeEvent` (`self.StateTreeAI`) (make `StateTreeEvent` (struct :`TagName` "State_Chase")))
      (else
        (`StateTreeComponent.SendStateTreeEvent` (`self.StateTreeAI`) (make `StateTreeEvent` (struct :`TagName` "State_Patrol")))))))

(fn `UserConstructionScript`
  (`parent.UserConstructionScript`))